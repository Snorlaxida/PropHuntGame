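; Player controller for the Prop Hunt mode that owns each local player's main HUD and relays game-state updates to it.
; BeginPlay creates W_MainHUD for the local player on a listen host or a remote client.
; Paired wrapper and OnClient events forward prop role, health, round timer, crosshair hits and the win screen to the HUD.
; A similar pair sets a StopShooting flag, exposed through CheckStopShooting.
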(event `self.ReceiveBeginPlay`
  ;[1 1 1] Create Widgets For Clients
  (`/Engine/EditorBlueprintResources/ActorMacros.Switch Has Authority`
    (:`Authority`
      (if (`self.IsLocalPlayerController`)
        (bind _returnvalue (`|CreateWidget` "/Game/Core/Widgets/W_MainHUD.W_MainHUD_C" self :!label _label))
        (bind _output_get (set `self.MainHUDRef` _returnvalue))
        (`UserWidget.AddToViewport` _output_get 0)))
    (:`Remote`
      (goto _label))))

(event `/Game/Core/Blueprints/Interfaces/BPI_PropHuntController.SetupPropWidget`
  (params (`IsProp?` :type Boolean))
  (bind _output_get (set `self.Is Prop?` `IsProp?`))
  (`self.SetPropOnClient` _output_get))

(event `SetPropOnClient`
  (params (`IsProp?` :type Boolean))
  (`/Game/Core/Widgets/W_MainHUD.SetupPropWidgets` (`self.MainHUDRef`) `IsProp?`))

(event `/Game/Core/Blueprints/Interfaces/BPI_PropHuntController.UpdateHealthWidget`
  (params (Health :type "Float (double-precision)"))
  (`self.UpdateHealthOnClient` Health))

(event `UpdateHealthOnClient`
  (params (Health :type "Float (double-precision)"))
  (`/Game/Core/Widgets/W_MainHUD.UpdateHealthBar` (`self.MainHUDRef`) Health))

(event `/Game/Core/Blueprints/Interfaces/BPI_PropHuntController.ShowWinScreenWidget`
  (params (`PropWon?` :type Boolean))
  (`self.ShowWinScreenOnClient` `PropWon?` (`self.Is Prop?`)))

(event `ShowWinScreenOnClient`
  (params (`PropWon?` :type Boolean) (`IsProp?` :type Boolean))
  (`/Game/Core/Widgets/W_MainHUD.ShowWinScreen` (`self.MainHUDRef`) `PropWon?` `IsProp?`))

(event `/Game/Core/Blueprints/Interfaces/BPI_PropHuntController.StartTimerWidget`
  (params (Time :type "Float (double-precision)"))
  (`self.StartTimerOnClient` Time))

(event `StartTimerOnClient`
  (params (Time :type "Float (double-precision)"))
  (`/Game/Core/Widgets/W_MainHUD.StartTimer` (`self.MainHUDRef`) Time))

(event `/Game/Core/Blueprints/Interfaces/BPI_PropHuntController.HitCrosshairWidget`
  (`self.HitCrosshairOnClient`))

(event `HitCrosshairOnClient`
  (`/Game/Core/Widgets/W_MainHUD.HitCrosshair` (`self.MainHUDRef`)))

(event `/Game/Core/Blueprints/Interfaces/BPI_PropHuntController.StopShooting`
  (`self.StopShootingOnClient`))

(event `StopShootingOnClient`
  (set `self.StopShooting?` true))

(fn `CheckStopShooting`
  (returns (`StopShoot?` :type Boolean))
  (return (`self.StopShooting?`)))

(fn `UserConstructionScript`)